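; BP_Coin1 is a coin item locked to the Y=0 plane by its construction script, as for a side-scroller.
; Its event graph holds pickup logic that never runs, as no live event connects to it.
; That disconnected logic casts to GameplayPC, then on authority plays a sound, destroys the coin and counts coins, granting a life past 100.
; The positional, attenuated coin sound sits in another disconnected chain.
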(event EventBeginPlay)

(event Collision|EventActorBeginOverlap
  (params (OtherActor :type Actor%20Object%20Reference)))

(event EventTick
  (params (DeltaSeconds :type Float%20%28single-precision%29)))

(fn ConstructionScript
  (bind _returnvalue (Transformation|GetActorLocation))
  (Transformation|SetActorLocation (Math|Vector|MakeVector (.x _returnvalue) 0.0 (.z _returnvalue)) false false) ; Keep on Y axes of 0
)