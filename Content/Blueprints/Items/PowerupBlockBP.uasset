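; PowerupBlockBP is a Mario-style item block that gives items when an airborne Base2DCharacter overlaps it.
; A hit bumps the sprite on a timeline while GiveItems spawns an ItemType actor above, animates it upward, applies its value and destroys it.
; Each payout decrements ItemsInBlock, and the empty block is destroyed by multicast from the authority.
; The construction script sets the block's location from its X and Z only.
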(event Custom|GiveItems
  (params (CharacterReference :type Base%202D%20Character%20Object%20Reference))
  (bind _self self)
  (bind _returnvalue (Transformation|GetActorTransform _self))
  (bind (_x _y _z) (Math|Vector|BreakVector (.location _returnvalue)))
  (Variables|Default|SetCharRef CharacterReference)
  (Utilities|FlowControl|DoOnce false :!label _label
    (:Completed
      (if (not (<= (Variables|Items|GetItemsInBlock) 0))
        (if (Variables|Default|GetbActive)
          (Variables|Default|SetbActive false)
          (bind _returnvalue_2 (Game|SpawnActorfromClass (Variables|Default|GetItemType) (Math|Transform|MakeTransform (Math|Vector|MakeVector _x _y (+ _z 1.2e+02)) (.rotation _returnvalue) (.scale _returnvalue)) "Undefined" (Variables|Default|GetCharRef) 0))
          (bind _output_get (Variables|Default|SetItemReference _returnvalue_2))
          (Variables|/Game/Blueprints/Items/ItemBase.ItemBase_C|SetbBobsUpAndDown _output_get false)
          (Utilities|FlowControl|Sequence
            (:then_0
              (bind _coinanimation (Timeline|CoinAnimation PlayFromStart)
                (:Update
                  (Transformation|SetActorRelativeLocation (Variables|Default|GetItemReference) (Math|Vector|Lerp(Vector) (Transformation|GetActorLocation (Variables|Default|GetItemReference)) (Math|Vector|MakeVector (.X (Math|Vector|BreakVector (Transformation|GetActorLocation (Variables|Default|GetItemReference)))) (.Y (Math|Vector|BreakVector (Transformation|GetActorLocation (Variables|Default|GetItemReference)))) (+ (.Z (Math|Vector|BreakVector (Transformation|GetActorLocation (Variables|Default|GetItemReference)))) 3e+01)) _coinanimation)))
                (:Finished
                  (if (not (<= (Variables|Items|GetItemsInBlock) 0))
                    (Variables|Items|SetItemsInBlock (- (Variables|Items|GetItemsInBlock) 1))
                    ;[1 1 1] Since this is using the ItemBase Custom Things For Spawned Item Don't Happen
                    (Default|AddItemValue (Variables|Default|GetItemReference) (Variables|Default|GetCharRef))
                    (Actor|DestroyActor (Variables|Default|GetItemReference))
                    (Utilities|FlowControl|Delay 0.1)
                    (Variables|Default|SetbActive true)
                    (goto _label Reset)))))))))))

(event Custom|MulticastDestroyMe
  (Actor|DestroyActor self))

(event Collision|EventActorBeginOverlap
  (params (OtherActor :type Actor%20Object%20Reference))
  (bind _asbase_2dcharacter (Utilities|Casting|CastToBase2DCharacter OtherActor))
  (Variables|Default|SetCharRef _asbase_2dcharacter)
  (Collision|SetCollisionEnabled (Variables|Default|GetCollision) "NoCollision")
  (if (and (AI|Components|NavMovement|IsFalling (Pawn|GetMovementComponent _asbase_2dcharacter)) (not (Variables|Default|GetHit)))
    (Variables|Default|SetHit true)
    (CallFunction|GiveItems (Variables|Default|GetCharRef))
    (bind _newtrack_0 (Timeline|Timeline_0 PlayFromStart)
      (:Update
        (Transformation|SetRelativeLocation (Variables|Default|GetBlockSprite) (Math|Vector|Lerp(Vector) "0, 0, 0" "0, 0,50.000000" _newtrack_0) false false))
      (:Finished
        (Variables|Default|SetHit false)
        (Utilities|FlowControl|Delay 0.2)
        (if (<= (Variables|Items|GetItemsInBlock) 0)
          (Networking|SwitchHasAuthority
            (:Authority
              (CallFunction|MulticastDestroyMe)))
          (else
            (Collision|SetCollisionEnabled (Variables|Default|GetCollision) "QueryOnly")))))))

(fn ConstructionScript
  (bind _returnvalue (Transformation|GetActorLocation))
  (Transformation|SetActorLocation (Math|Vector|MakeVector (.x _returnvalue) 0.0 (.z _returnvalue)) false false))