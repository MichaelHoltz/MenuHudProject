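; Item respawner actor that spawns a random class from its ItemsToSpawn list at a spawn point.
; On BeginPlay it either spawns an item immediately or sets a SpawnItem timer, depending on StartsWithItem and HasItem.
; On the authority, a Base2DCharacter entering the box clears HasItem without checking for an actual pickup.
; Leaving the box while HasItem is false starts a fixed-delay respawn timer.
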(event OnComponentEndOverlap(Box)
  (params (OverlappedComponent :type Primitive%20Component%20Object%20Reference) (OtherActor :type Actor%20Object%20Reference) (OtherComp :type Primitive%20Component%20Object%20Reference) (OtherBodyIndex :type Integer))
  (Networking|SwitchHasAuthority
    (:Authority
      (Utilities|Casting|CastToBase2DCharacter OtherActor)
      (if (not (Variables|Default|GetHasItem?))
        (Variables|Default|SetTimeDelay 5.0)
        (Utilities|Time|SetTimerbyFunctionName 0 "SpawnItem" (Variables|Default|GetTimeDelay))
        (Development|PrintString "Timer Unpaused")))))

(event OnComponentBeginOverlap(Box)
  (params (OverlappedComponent :type Primitive%20Component%20Object%20Reference) (OtherActor :type Actor%20Object%20Reference) (OtherComp :type Primitive%20Component%20Object%20Reference) (OtherBodyIndex :type Integer) (bFromSweep :type Boolean) (SweepResult :type Hit%20Result%20Structure%20%28by%20ref%29))
  (Networking|SwitchHasAuthority
    (:Authority
      (Utilities|Casting|CastToBase2DCharacter OtherActor)
      (Variables|Default|SetHasItem? false))))

(event Custom|SpawnItem
  (Development|PrintString "Spawning Item" true true "(R=0.000000,G=0.660000,B=1.000000,A=1.000000)" 1e+01)
  (bind _newparam (CallFunction|GetItemtoSpawn))
  (Game|SpawnActorfromClass _newparam (Math|Conversions|ToTransform(Vector) (Transformation|GetWorldLocation (Variables|Default|GetSpawnPoint))) "Undefined" 0 0)
  (Variables|Default|SetHasItem? true))

(event EventBeginPlay
  (Networking|SwitchHasAuthority
    (:Authority
      _)
    (:Remote
      _))
  (if (Variables|Default|GetStartsWithItem?)
    (if (Variables|Default|GetHasItem?)
      (Utilities|Time|SetTimerbyFunctionName 0 "SpawnItem" (Variables|Default|GetTimeDelay) :!label _label)
      (else
        (bind _newparam (CallFunction|GetItemtoSpawn))
        (Game|SpawnActorfromClass _newparam (Math|Conversions|ToTransform(Vector) (Transformation|GetWorldLocation (Variables|Default|GetSpawnPoint))) "Undefined" 0 0)
        (Variables|Default|SetHasItem? true)))
    (else
      (goto _label))))

(event Collision|EventActorBeginOverlap
  (params (OtherActor :type Actor%20Object%20Reference)))

(event EventTick
  (params (DeltaSeconds :type Float%20%28single-precision%29)))

(fn ConstructionScript)

(fn GetItemtoSpawn
  (bind _itemstospawn (Variables|ItemProperties|GetItemsToSpawn))
  (return (Utilities|Array|Get(acopy) _itemstospawn (Math|Random|RandomIntegerinRange 0 (- (Utilities|Array|Length _itemstospawn) 1)))))