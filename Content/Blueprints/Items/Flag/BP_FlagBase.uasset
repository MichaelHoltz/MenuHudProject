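; BP_FlagBase is a capturable flag pickup for a 2D game, pinned to the Y=0 plane by its construction script.
; A cooldown timer started at BeginPlay enables capture and sets the sprite color to white.
; An overlapping Base2DCharacter then gets a BP_FlagIcon attached to its sprite's HatSocket.
; If that character has a GameplayPC controller, it receives capture force feedback and the flag destroys itself.
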(event Custom|EnableCapture
  (Variables|Default|SetCanBeCaptured? true)
  (Sprite|SetSpriteColor (Variables|Default|GetPaperSprite) "(R=1.000000,G=1.000000,B=1.000000,A=1.000000)"))

(event Custom|PlayFeedbackOnClient
  (params (TheActor :type Actor%20Object%20Reference))
  (bind _asbase_2dcharacter (Utilities|Casting|CastToBase2DCharacter TheActor))
  (bind _asgameplay_pc (Utilities|Casting|CastToGameplayPC (Pawn|GetController _asbase_2dcharacter)))
  (Game|Feedback|ClientPlayForceFeedback _asgameplay_pc "/Game/Blueprints/Items/Flag/FlagCaptureFFEA.FlagCaptureFFEA" false "None")
  (Development|PrintString (Utilities|String|Append "BP_FlagBase - Play Force Feedback on: " (Utilities|GetObjectName _asbase_2dcharacter)) true true "(R=0.000000,G=0.660000,B=1.000000,A=1.000000)" 1e+01))

(event EventBeginPlay
  (Utilities|Time|SetTimerbyEvent (delegate Custom|EnableCapture) (Variables|Default|GetCoolDownTime)))

(event Collision|EventActorBeginOverlap
  (params (OtherActor :type Actor%20Object%20Reference))
  (if (Variables|Default|GetCanBeCaptured?)
    (bind _output_get (Variables|Default|SetOtherActorRef OtherActor))
    (bind _asbase_2dcharacter (Utilities|Casting|CastToBase2DCharacter _output_get))
    (bind _returnvalue (Game|SpawnActorfromClass "/Game/Blueprints/Items/Flag/BP_FlagIcon.BP_FlagIcon_C" (Math|Transform|MakeTransform (Math|Vector|MakeVector (.x (Transformation|GetActorLocation _asbase_2dcharacter)) 0.0 (.z (Transformation|GetActorLocation _asbase_2dcharacter))) (Math|Rotator|MakeRotator (.roll (Transformation|GetActorRotation _asbase_2dcharacter)) (.pitch (Transformation|GetActorRotation _asbase_2dcharacter)) (- (.yaw (Transformation|GetActorRotation _asbase_2dcharacter)) 1.8e+02)) "1,1,1") "Undefined" (Variables|Default|GetOtherActorRef) 0))
    (Transformation|AttachComponentToComponent _returnvalue (Variables|/Script/Paper2D.PaperCharacter|GetSprite _asbase_2dcharacter) "HatSocket" "SnapToTarget" "KeepWorld" "SnapToTarget" true)
    ;[1 1 1] Seems to only play on the Server - But maybe needs testing on seperate computer
    (Utilities|Casting|CastToGameplayPC (Pawn|GetController _asbase_2dcharacter))
    (CallFunction|PlayFeedbackonClient (Variables|Default|GetOtherActorRef))
    (Actor|DestroyActor)))

(event EventTick
  (params (DeltaSeconds :type Float%20%28single-precision%29)))

(fn ConstructionScript
  (bind _returnvalue (Transformation|GetActorLocation))
  ;[1 1 1] Auto Snap to Y axis
  (Transformation|SetActorLocation (Math|Vector|MakeVector (.x _returnvalue) 0.0 (.z _returnvalue)) false false) ; Keep on Y axis of 0
)