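; Base pickup item that grants points, health or energy by item type when overlapped, then plays a sound and destroys itself.
; Server-only collection accepts projectiles if shootable, enemies if allowed, or actors with a gameplay player controller as instigator.
; Rewards go to the stored controller reference, which only the player branch sets.
; Construction snaps it to the Y=0 plane and applies flipbook, sprite and particles; bobbing logic is unconnected.
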(event Custom|PlaySound
  ;[1 1 1] Play DestroySound at this Item location
  (Audio|PlaySoundatLocation (Variables|ItemSettings|GetDestroySound) (Transformation|GetActorLocation self) "0, 0, 0" 1.0 1.0 0.0 "/Game/Blueprints/Items/ItemAttenuation.ItemAttenuation"))

(event EventBeginPlay)

(event EventTick
  (params (DeltaSeconds :type Float%20%28single-precision%29)))

(event Collision|EventActorBeginOverlap
  (params (OtherActor :type Actor%20Object%20Reference))
  (bind _myitemvalue (Variables|ItemSettings|GetMyItemValue))
  ;[1 1 1] get player controller from other actor
  (Utilities|Casting|CastToProjectile OtherActor
    (:then
      (if (Variables|ItemSettings|GetbCanBeShot)
        ;[1 1 1] Play sound at actor location
        (Networking|SwitchHasAuthority :!label _label
          (:Authority
            (CallFunction|PlaySound)
            ;[1 1 1] Kill the Item
            (Actor|DestroyActor self)
            ;[1 1 1] Set Item Value
            (switch Utilities|FlowControl|Switch|SwitchonItemType (Variables|ItemSettings|GetMyItemType)
              (:NewEnumerator0
                (Default|AddPoints (Variables|ItemSettings|GetGamePlayControllerRef) _myitemvalue))
              (:NewEnumerator1
                (Default|AddHealth (Variables|ItemSettings|GetGamePlayControllerRef) _myitemvalue))
              (:NewEnumerator2
                (Default|AddEnergy (Variables|ItemSettings|GetGamePlayControllerRef) _myitemvalue)))))))
    (:CastFailed
      (Utilities|Casting|CastToEnemy OtherActor
        (:then
          (if (Variables|ItemSettings|GetbEnemyCanTake)
            (goto _label)))
        (:CastFailed
          (bind _asgameplay_pc (Utilities|Casting|CastToGameplayPC (Game|GetInstigatorController OtherActor)))
          (Variables|ItemSettings|SetGamePlayControllerRef _asgameplay_pc)
          (goto _label))))))

(fn ConstructionScript
  (bind _returnvalue (Transformation|GetActorLocation))
  ;[1 1 1] Auto Snap to Y axis
  (Transformation|SetActorLocation (Math|Vector|MakeVector (.x _returnvalue) 0.0 (.z _returnvalue)) false false) ; Keep on Y axis of 0
  ;[1 1 1] Set Specificlly chosen settings for this item
  (Sprite|SetFlipbook (Variables|Default|GetItemFlipbook) (Variables|ItemSettings|GetMyFlipBook))
  (Rendering|Components|Sprite|SetSprite (Variables|Default|GetItemSprite) (Variables|ItemSettings|GetMySprite))
  (Effects|Components|ParticleSystem|SetTemplate (Variables|Default|GetItemParticleSystem) (Variables|ItemSettings|GetMyParticleSystem)))