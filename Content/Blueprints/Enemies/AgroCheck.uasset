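; Behavior tree aggro check that finds visible targets around an AI-controlled enemy on each tick.
; It caches the MyAIController, then sphere-traces around its pawn, ignoring all RedBoxyCharacter_Enemy actors.
; A camera-channel line trace tests sight to each hit, setting TargetToFollow and TargetLocation or clearing TargetToFollow when blocked.
; The last hit processed wins, and an empty sweep leaves the blackboard unchanged.
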(event EventTick
  (params (OwnerActor :type Actor%20Object%20Reference) (DeltaSeconds :type Float%20%28single-precision%29))
  (if (!= (Variables|Default|GetAI_CON_Ref) 0)
    _
    (else
      (bind _asmy_aicontroller (Utilities|Casting|CastToMyAIController OwnerActor))
      (Variables|Default|SetAI_CON_Ref _asmy_aicontroller)))
  (bind _outactors (Actor|GetAllActorsOfClass "/Game/Blueprints/Characters/RedBoxyCharacter_Enemy.RedBoxyCharacter_Enemy_C"))
  (Variables|Default|SetMyLocation (Transformation|GetActorLocation (Pawn|GetControlledPawn (Variables|Default|GetAI_CON_Ref))))
  (bind _outhits (Collision|MultiSphereTraceForObjects (Transformation|GetActorLocation (Pawn|GetControlledPawn (Variables|Default|GetAI_CON_Ref))) (+ (Transformation|GetActorLocation (Pawn|GetControlledPawn (Variables|Default|GetAI_CON_Ref))) "0, 0,15.000000") 3e+02 (Variables|Default|GetDesiredObjectTypes) false _outactors "None"))
  (bind _array_element (Utilities|Array|ForEachLoopwithBreak _outhits)
    (:LoopBody
      (bind _outhit (Collision|LineTraceByChannel (Variables|Default|GetMyLocation) (Transformation|GetActorLocation (.HitActor (Collision|BreakHitResult _array_element))) "TraceTypeQuery2" false _outactors "ForDuration"))
      (if (== (.HitActor (Collision|BreakHitResult _outhit)) (.HitActor (Collision|BreakHitResult _array_element)))
        (Class|BTFunctionLibrary|SetBlackboardValueasObject (Variables|Default|GetTargetToFollow) (.HitActor (Collision|BreakHitResult _outhit)))
        (AI|BehaviorTree|SetBlackboardValueasVector (Variables|Default|GetTargetLocation) (Transformation|GetActorLocation (.HitActor (Collision|BreakHitResult _outhit))))
        (else
          (Class|BTFunctionLibrary|SetBlackboardValueasObject (Variables|Default|GetTargetToFollow)))))))