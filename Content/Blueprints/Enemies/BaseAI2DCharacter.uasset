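; Base 2D AI enemy character that turns to face its movement direction and applies damage to Base2DCharacter actors it hits.
; On authority, Tick sets controller yaw from the sign of X velocity, keeping the last facing when stopped; a comment notes morphing still misbehaves.
; Capsule hits apply a small negative damage value.
; Jump input triggers a jump only when the controller is MyAIController.
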(event OnComponentHit(CapsuleComponent)
  (params (HitComponent :type Primitive%20Component%20Object%20Reference) (OtherActor :type Actor%20Object%20Reference) (OtherComp :type Primitive%20Component%20Object%20Reference) (NormalImpulse :type Vector :default "0, 0, 0") (Hit :type Hit%20Result%20Structure%20%28by%20ref%29))
  (bind _asbase_2dcharacter (Utilities|Casting|CastToBase2DCharacter OtherActor))
  (Game|Damage|ApplyDamage _asbase_2dcharacter -0.1 0 self))

(event EventBeginPlay)

(event Collision|EventActorBeginOverlap
  (params (OtherActor :type Actor%20Object%20Reference)))

(event EventTick
  (params (DeltaSeconds :type Float%20%28single-precision%29))
  ;[1 1 1] Tick - Updates animation - added mess is to avoid error when morphing but is still not working right for morphing
  (Networking|SwitchHasAuthority
    (:Authority
      (Math|Float|CompareFloat (.X (Math|Vector|BreakVector (Variables|/Script/Engine.MovementComponent|GetVelocity (Pawn|GetMovementComponent)))) 0.0
        (:>
          (Variables|Default|SetbisMovingRight true)
          (Pawn|SetControlRotation (Pawn|GetController) (Math|Rotator|MakeRotator 0.0 0.0 0.0) :!label _label))
        (:==
          (if (Variables|Default|GetbisMovingRight)
            (goto _label)
            (else
              (Pawn|SetControlRotation (Pawn|GetController) (Math|Rotator|MakeRotator 0.0 0.0 1.8e+02) :!label _label_2))))
        (:<
          (Variables|Default|SetbisMovingRight false)
          (goto _label_2)))
      (if (AI|Components|NavMovement|IsFalling (Variables|Character|GetCharacterMovement self))
        _))))

(event Input|ActionEvents|InputActionJump
  (params (Key :type Key%20Structure :default "AnyKey"))
  ;[1 1 1] Handle Jump
  (:Pressed
    (bind _returnvalue (AI|GetAIController self))
    (Utilities|Casting|CastToMyAIController _returnvalue)
    (Character|Jump))
  (:Released
    (Character|StopJumping)))

(fn ConstructionScript)