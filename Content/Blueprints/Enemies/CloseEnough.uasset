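; CloseEnough is a behavior tree decorator for enemy AI that gates a branch on distance to a follow target.
; It casts the owner to MyAIController and measures the distance from its controlled pawn to the TargetToFollow blackboard actor.
; Despite its name, it passes when that distance is at or beyond AcceptanceDistance.
; A debug print of the result is left unconnected.
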(fn PerformConditionCheck
  (params (OwnerActor :type Actor%20Object%20Reference))
  (bind _asmy_aicontroller (Utilities|Casting|CastToMyAIController OwnerActor))
  (Variables|Default|SetAI_CON_Ref _asmy_aicontroller)
  (return (>= (Math|Vector|VectorLength (- (Transformation|GetActorLocation (AI|BehaviorTree|GetBlackboardValueasActor (Variables|Default|GetTargetToFollow))) (Transformation|GetActorLocation (Pawn|GetControlledPawn (Variables|Default|GetAI_CON_Ref))))) (Variables|Default|GetAcceptanceDistance))))