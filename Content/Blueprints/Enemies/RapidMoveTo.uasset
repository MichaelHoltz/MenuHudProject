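; Behavior Tree task for 2D enemy AI that moves the controlled pawn to the TargetToFollow blackboard actor.
; It caches the MyAIController on first execution, then runs AI MoveTo, finishing as failed even when the move succeeds.
; On move failure, the BaseAI2DCharacter jumps with a velocity impulse toward the target and TargetToFollow is cleared.
; The failure path never calls FinishExecute.
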(event EventReceiveExecute
  (params (OwnerActor :type Actor%20Object%20Reference))
  (bind _targettofollow (Variables|Default|GetTargetToFollow))
  (bind _returnvalue (AI|BehaviorTree|GetBlackboardValueasActor _targettofollow))
  (if (!= (Variables|Default|GetAI_CON_Ref) 0)
    _
    (else
      (bind _asmy_aicontroller (Utilities|Casting|CastToMyAIController OwnerActor))
      (Variables|Default|SetAI_CON_Ref _asmy_aicontroller)))
  (AI|AIMoveTo (Pawn|GetControlledPawn (Variables|Default|GetAI_CON_Ref)) "0, 0, 0" _returnvalue 5e+01 false
    (:OnSuccess
      (AI|BehaviorTree|FinishExecute false))
    (:OnFail
      (bind _asbase_ai2dcharacter (Utilities|Casting|CastToBaseAI2DCharacter (Pawn|GetControlledPawn (Variables|Default|GetAI_CON_Ref)))
        (:then
          (Character|Jump _asbase_ai2dcharacter)
          (Utilities|IsValid (Variables|/Script/Engine.Character|GetCharacterMovement _asbase_ai2dcharacter)
            (:Is%20Valid
              (Physics|AddImpulse (Variables|/Script/Engine.Character|GetCharacterMovement _asbase_ai2dcharacter) (- (Transformation|GetActorLocation _returnvalue) (Transformation|GetActorLocation _asbase_ai2dcharacter)) true))
            (:Is%20Not%20Valid
              _)))
        (:CastFailed
          _))
      (Class|BTFunctionLibrary|SetBlackboardValueasObject (Variables|Default|GetTargetToFollow)))))