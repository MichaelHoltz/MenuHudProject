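; Tennis ball projectile for the 2D game that destroys itself when its movement stops and passes over items without effect on hit.
; Hitting a character other than its instigator applies a small negative damage value, a velocity-based knockback impulse and controller force feedback through the player's GameplayPC.
; Enemies instead receive their own Damage call.
; Both kinds of hit spawn an explosion puff and destroy the ball.
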(event OnProjectileStop(ProjectileMovement)
  (params (ImpactResult :type Hit%20Result%20Structure%20%28by%20ref%29))
  ;[1 1 1] Destroy Tennis Ball When it stops Moving
  (Actor|DestroyActor))

(event OnComponentHit(Sphere)
  (params (HitComponent :type Primitive%20Component%20Object%20Reference) (OtherActor :type Actor%20Object%20Reference) (OtherComp :type Primitive%20Component%20Object%20Reference) (NormalImpulse :type Vector :default "0, 0, 0") (Hit :type Hit%20Result%20Structure%20%28by%20ref%29))
  (bind _returnvalue (Transformation|GetVelocity))
  (bind _self self)
  (bind _returnvalue_2 (Game|GetInstigator _self))
  (Utilities|Casting|CastToItemBase OtherActor ; If Item I shootable
    (:CastFailed
      ;[1 1 1] Don't Shoot Self
      (bind _asbase_2dcharacter (Utilities|Casting|CastToBase2DCharacter OtherActor)
        (:then
          (if (not (== _asbase_2dcharacter _returnvalue_2))
            (Game|Damage|ApplyDamage _asbase_2dcharacter -0.1 0 _returnvalue_2)
            (CallFunction|PlayFeedbackonClient _asbase_2dcharacter)
            (Physics|AddImpulse (Variables|/Script/Engine.Character|GetCharacterMovement _asbase_2dcharacter) (Math|Vector|MakeVector (/ (.x _returnvalue) 2.0) 0.0 (.z _returnvalue)) true)
            (Game|SpawnActorfromClass "/Game/Blueprints/Projectiles/TennisBallExplodyPuff.TennisBallExplodyPuff_C" (Math|Conversions|ToTransform(Vector) (Transformation|GetActorLocation)) "AdjustIfPossibleButDontSpawnIfColliding" 0 0 :!label _label)
            (Actor|DestroyActor)))
        (:CastFailed
          (bind _asenemy (Utilities|Casting|CastToEnemy OtherActor))
          (Default|Damage _asenemy (Variables|Default|GetDamageAmount))
          (goto _label))))))

(event Custom|PlayFeedbackOnClient
  (params (TheActor :type Actor%20Object%20Reference))
  (bind _asbase_2dcharacter (Utilities|Casting|CastToBase2DCharacter TheActor))
  (bind _asgameplay_pc (Utilities|Casting|CastToGameplayPC (Pawn|GetController _asbase_2dcharacter)))
  (Game|Feedback|ClientPlayForceFeedback _asgameplay_pc "/Game/Blueprints/Items/Flag/FlagCaptureFFEA.FlagCaptureFFEA" false "None")
  (Development|PrintString (Utilities|String|Append "BP_TennisBall - Play Force Feedback on: " (Utilities|GetObjectName _asbase_2dcharacter)) true true "(R=0.000000,G=0.660000,B=1.000000,A=1.000000)" 1e+01))

(event Custom|CustomEvent
  (params (OtherActor :type Actor%20Object%20Reference)))

(event EventBeginPlay)

(event Collision|EventActorBeginOverlap
  (params (OtherActor :type Actor%20Object%20Reference)))

(event EventTick
  (params (DeltaSeconds :type Float%20%28single-precision%29)))

(fn ConstructionScript
  (AddComponent|AddPaperFlipbookComponent false (Math|Transform|MakeTransform "0.000000,0.000000,0.000000" "0, 0, 0" "1.000000,1.000000,1.000000")))