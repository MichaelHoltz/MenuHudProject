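; Base projectile for a game with 2D characters that damages characters and enemies and plays sounds for firing, flight, impact and death.
; Sphere hits branch by type: characters other than the instigator take damage, a velocity-based impulse and controller rumble, while enemies receive their own Damage call.
; Both then spawn a destroy effect and remove the projectile.
; Items and other surfaces only trigger one-shot sounds, and the projectile destroys itself when movement stops.
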(event OnProjectileStop(ProjectileMovement)
  (params (ImpactResult :type Hit%20Result%20Structure%20%28by%20ref%29))
  ;[1 1 1] Destroy  When it stops Moving
  (Utilities|FlowControl|DoOnce false
    (:Completed
      (CallFunction|PlaySound (Variables|Default|GetDeathSounds))
      (Actor|DestroyActor))))

(event OnProjectileBounce(ProjectileMovement)
  (params (ImpactResult :type Hit%20Result%20Structure%20%28by%20ref%29) (ImpactVelocity :type Vector%20%28by%20ref%29 :default "0, 0, 0")))

(event OnComponentHit(Sphere)
  (params (HitComponent :type Primitive%20Component%20Object%20Reference) (OtherActor :type Actor%20Object%20Reference) (OtherComp :type Primitive%20Component%20Object%20Reference) (NormalImpulse :type Vector :default "0, 0, 0") (Hit :type Hit%20Result%20Structure%20%28by%20ref%29))
  (bind _returnvalue (Transformation|GetVelocity))
  (bind _self self)
  (bind _returnvalue_2 (Game|GetInstigator _self))
  (bind _asitem_base (Utilities|Casting|CastToItemBase OtherActor) ; If Item I shootable
    (:then
      (if (Variables|/Game/Blueprints/Items/ItemBase.ItemBase_C|GetbCanBeShot _asitem_base)
        (Utilities|FlowControl|DoOnce false
          (:Completed
            (CallFunction|PlaySound (Variables|Default|GetMissSounds))))
        (else
          (Utilities|FlowControl|DoOnce false
            (:Completed
              (CallFunction|PlaySound (Variables|Default|GetHurtSounds)))))))
    (:CastFailed
      ;[1 1 1] Don't Shoot Self
      (bind _asbase_2dcharacter (Utilities|Casting|CastToBase2DCharacter OtherActor)
        (:then
          (if (not (== _asbase_2dcharacter _returnvalue_2))
            (Game|Damage|ApplyDamage _asbase_2dcharacter (Variables|Default|GetDamageAmount) 0 _returnvalue_2)
            (CallFunction|PlayFeedbackonClient _asbase_2dcharacter)
            (Physics|AddImpulse (Variables|/Script/Engine.Character|GetCharacterMovement _asbase_2dcharacter) (Math|Vector|MakeVector (/ (.x _returnvalue) 2.0) 0.0 (.z _returnvalue)) true)
            (Utilities|FlowControl|DoOnce false :!label _label
              (:Completed
                (CallFunction|PlaySound (Variables|Default|GetDeathSounds))
                (CallFunction|DestroyMe)))))
        (:CastFailed
          (bind _asenemy (Utilities|Casting|CastToEnemy OtherActor)
            (:then
              (Default|Damage _asenemy (Variables|Default|GetDamageAmount))
              (goto _label))
            (:CastFailed
              (Utilities|FlowControl|DoOnce false
                (:Completed
                  (CallFunction|PlaySound (Variables|Default|GetMissSounds)))))))))))

(event Custom|PlaySound
  (params (SoundWaveArray :type Array%20of%20Sound%20Wave%20Object%20References))
  (if (Utilities|Array|IsValidIndex SoundWaveArray)
    (Audio|PlaySoundatLocation (Utilities|Array|Get(acopy) SoundWaveArray (Math|Random|RandomIntegerinRange 0 (- (Utilities|Array|Length SoundWaveArray) 1))) (Transformation|GetActorLocation self) "0, 0, 0" 1.0 1.0 0.0 "/Game/Blueprints/Items/ItemAttenuation.ItemAttenuation")))

(event Custom|PlayFeedbackOnClient
  (params (TheActor :type Actor%20Object%20Reference))
  (bind _asbase_2dcharacter (Utilities|Casting|CastToBase2DCharacter TheActor))
  (bind _asgameplay_pc (Utilities|Casting|CastToGameplayPC (Pawn|GetController _asbase_2dcharacter)))
  (Game|Feedback|ClientPlayForceFeedback _asgameplay_pc "/Game/Blueprints/Items/Flag/FlagCaptureFFEA.FlagCaptureFFEA" false "None"))

(event Custom|DestroyMe
  (Game|SpawnActorfromClass (Variables|Default|GetDestroyEffect) (Math|Conversions|ToTransform(Vector) (Transformation|GetActorLocation)) "AdjustIfPossibleButDontSpawnIfColliding" 0 0)
  (Actor|DestroyActor))

(event EventBeginPlay
  (Utilities|FlowControl|DoOnce false
    (:Completed
      (CallFunction|PlaySound (Variables|Default|GetFireSounds))
      (Utilities|FlowControl|DoOnce false
        (:Completed
          (CallFunction|PlaySound (Variables|Default|GetFlyingSounds)))))))

(event Collision|EventActorBeginOverlap
  (params (OtherActor :type Actor%20Object%20Reference)))

(event EventTick
  (params (DeltaSeconds :type Float%20%28single-precision%29)))

(fn ConstructionScript)