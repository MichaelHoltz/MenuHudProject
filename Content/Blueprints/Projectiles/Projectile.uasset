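; Fireball projectile with a Paper2D flipbook visual and an attached trail emitter, which resolves its hit on actor overlap.
; Enemies receive its damage amount, while 2D characters other than the instigator get a small, negative-valued ApplyDamage call.
; It spawns an explosion puff and destroys itself on any overlap, including items, except with the instigating character, which it ignores.
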(event EventBeginPlay
  (Effects|SpawnEmitterAttached "/Game/Effects/FireballTrail.FireballTrail" (Variables|Default|GetTrailAttach) "None" "0,0.000000, 0" "0, 0, 0" "SnapToTarget"))

(event Collision|EventActorBeginOverlap
  (params (OtherActor :type Actor%20Object%20Reference))
  (bind _self self)
  (bind _returnvalue (Game|GetInstigator _self))
  (Utilities|Casting|CastToItemBase OtherActor ; If Item I shootable
    (:then
      (Game|SpawnActorfromClass "/Game/Blueprints/Projectiles/ExplodyPuff.ExplodyPuff_C" (Math|Conversions|ToTransform(Vector) (Transformation|GetActorLocation)) "AdjustIfPossibleButDontSpawnIfColliding" 0 0 :!label _label)
      (Actor|DestroyActor))
    (:CastFailed
      ;[1 1 1] Don't Shoot Self
      (bind _asbase_2dcharacter (Utilities|Casting|CastToBase2DCharacter OtherActor)
        (:then
          (if (not (== _asbase_2dcharacter _returnvalue))
            (Game|Damage|ApplyDamage _asbase_2dcharacter -0.1 0 _returnvalue)
            (goto _label)))
        (:CastFailed
          (bind _asenemy (Utilities|Casting|CastToEnemy OtherActor)
            (:then
              (Default|Damage _asenemy (Variables|Default|GetDamageAmount))
              (goto _label))
            (:CastFailed
              (goto _label))))))))

(fn ConstructionScript
  (AddComponent|AddPaperFlipbookComponent false (Math|Transform|MakeTransform "-30.000000,0.000000,5.000000" "0, 0, 0" "1.500000,1.500000,1.500000")))