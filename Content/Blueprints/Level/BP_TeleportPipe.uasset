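; Warp pipe for a 2D game that teleports a Base2DCharacter to a linked pipe.
; On a start pipe, authority Tick detects a crouching character on top, disables input and slides TopGate aside.
; Hitting the bottom teleports the character to DestinationPipe, or, without one, launches it upward and re-enables input; rising out of the step trigger closes the gate.
; The construction script snaps the pipe to Y=0 and applies its sprite and flipbook.
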(event OnComponentBeginOverlap(StepTrigger)
  (params (OverlappedComponent :type Primitive%20Component%20Object%20Reference) (OtherActor :type Actor%20Object%20Reference) (OtherComp :type Primitive%20Component%20Object%20Reference) (OtherBodyIndex :type Integer) (bFromSweep :type Boolean) (SweepResult :type Hit%20Result%20Structure%20%28by%20ref%29))
  ;[1 1 1] Step On Step Trigger Event
  (bind _asbase_2dcharacter (Utilities|Casting|CastToBase2DCharacter OtherActor)
    (:then
      (Variables|Default|SetPlayerOnMe _asbase_2dcharacter)
      (Variables|Default|SetPlayerOnTop true))
    (:CastFailed
      (Variables|Default|SetPlayerOnMe 0)
      (Variables|Default|SetPlayerOnTop false))))

(event OnComponentEndOverlap(StepTrigger)
  (params (OverlappedComponent :type Primitive%20Component%20Object%20Reference) (OtherActor :type Actor%20Object%20Reference) (OtherComp :type Primitive%20Component%20Object%20Reference) (OtherBodyIndex :type Integer))
  ;[1 1 1] End of Exit Pipe
  (bind _asbase_2dcharacter (Utilities|Casting|CastToBase2DCharacter OtherActor))
  (Variables|Default|SetPlayerOnMe _asbase_2dcharacter)
  (Variables|Default|SetPlayerOnTop false)
  (if (> (.z (Transformation|GetVelocity _asbase_2dcharacter)) 0.0)
    (Networking|SwitchHasAuthority
      (:Authority
        (CallFunction|CloseTrapDoor)))))

(event OnComponentHit(BottomTrigger)
  (params (HitComponent :type Primitive%20Component%20Object%20Reference) (OtherActor :type Actor%20Object%20Reference) (OtherComp :type Primitive%20Component%20Object%20Reference) (NormalImpulse :type Vector :default "0, 0, 0") (Hit :type Hit%20Result%20Structure%20%28by%20ref%29))
  (bind _destinationpipe (Variables|Default|GetDestinationPipe))
  ;[1 1 1] After Teleport  - Spitting out the Player
  (bind _asbase_2dcharacter (Utilities|Casting|CastToBase2DCharacter OtherActor))
  (if (Utilities|IsValid _destinationpipe)
    (CallFunction|CloseTrapDoor)
    (Collision|SetActorEnableCollision _asbase_2dcharacter false)
    (Transformation|Teleport _asbase_2dcharacter (Transformation|GetWorldLocation (Variables|BP_TeleportPipe_C|GetTeleportDestination _destinationpipe)) "0, 0, 0")
    (Collision|SetActorEnableCollision _asbase_2dcharacter true)
    (else
      ;;[1 1 1] Open Trap Door and Spit out the Player
      (CallFunction|OpenTrapDoor)
      (Physics|AddImpulse (Variables|/Script/Engine.Character|GetCharacterMovement _asbase_2dcharacter) "0, 0,700.000000" true)
      (Utilities|FlowControl|Delay 0.5)
      (Input|EnableInput _asbase_2dcharacter 0))))

(event OnComponentBeginOverlap(StopDangerTrigger)
  (params (OverlappedComponent :type Primitive%20Component%20Object%20Reference) (OtherActor :type Actor%20Object%20Reference) (OtherComp :type Primitive%20Component%20Object%20Reference) (OtherBodyIndex :type Integer) (bFromSweep :type Boolean) (SweepResult :type Hit%20Result%20Structure%20%28by%20ref%29))
  ;[1 1 1] Can Enable or Disable any danger enemy that could be popping up and down
)

(event OnComponentEndOverlap(StopDangerTrigger)
  (params (OverlappedComponent :type Primitive%20Component%20Object%20Reference) (OtherActor :type Actor%20Object%20Reference) (OtherComp :type Primitive%20Component%20Object%20Reference) (OtherBodyIndex :type Integer))
  ;[1 1 1] Can Enable or Disable any danger enemy that could be popping up and down
)

(event Custom|OpenTrapDoor
  (bind _topgate (Variables|Default|GetTopGate))
  (bind _returnvalue (Transformation|GetWorldLocation _topgate))
  ;[1 1 1] Open the Trap Door to let Player In and Out
  (if (not (Variables|Default|GetMyTrapDoorIsOpen))
    (Variables|Default|SetStartingTrapDoorLocation (Transformation|GetWorldLocation _topgate))
    (Transformation|SetWorldLocation _topgate (Math|Vector|MakeVector (.x _returnvalue) (+ (.y _returnvalue) -1.5e+02) (.z _returnvalue)) false true)
    (Variables|Default|SetMyTrapDoorIsOpen true)))

(event Custom|ReleaseTrapDoor
  (bind _topgate (Variables|Default|GetTopGate))
  (bind _returnvalue (Transformation|GetWorldLocation _topgate))
  ;[1 1 1] Open the Trap Door to let Player In and Out
  (if (not (Variables|Default|GetMyTrapDoorIsOpen))
    (Variables|Default|SetStartingTrapDoorLocation (Transformation|GetWorldLocation _topgate))
    (Transformation|SetWorldLocation _topgate (Math|Vector|MakeVector (.x _returnvalue) (+ (.y _returnvalue) -1.5e+02) (.z _returnvalue)) false true)
    (Variables|Default|SetMyTrapDoorIsOpen true)))

(event Custom|CloseTrapDoor
  ;[1 1 1] Close the Trap Door to allow Stepping on it
  (if (Variables|Default|GetMyTrapDoorIsOpen)
    (Transformation|SetWorldLocation (Variables|Default|GetTopGate) (Variables|Default|GetStartingTrapDoorLocation) false true)
    (Variables|Default|SetMyTrapDoorIsOpen false)))

(event EventBeginPlay)

(event Collision|EventActorBeginOverlap
  (params (OtherActor :type Actor%20Object%20Reference)))

(event EventTick
  (params (DeltaSeconds :type Float%20%28single-precision%29))
  (Networking|SwitchHasAuthority
    (:Authority
      ;[1 1 1] No Entry unless TP Start
      (if (Variables|Default|GetIsTeleportStart)
        ;[1 1 1] Is Player On Top?
        (if (Variables|Default|GetPlayerOnTop)
          ;[1 1 1] Is Player Crouching
          (if (Variables|/Game/Blueprints/Characters/Base2DCharacter.Base2DCharacter_C|GetisCrouching (Variables|Default|GetPlayerOnMe))
            (Input|DisableInput 0)
            (CallFunction|ReleaseTrapDoor)
            (Variables|Default|SetPlayerOnTop false)))))))

(fn ConstructionScript
  (bind _returnvalue (Transformation|GetActorLocation))
  ;[1 1 1] Auto Snap to Y axis
  (Transformation|SetActorLocation (Math|Vector|MakeVector (.x _returnvalue) 0.0 (.z _returnvalue)) false false) ; Keep on Y axis of 0
  ;[1 1 1] Set Specificlly chosen Visual settings for this Pipe Teleporter
  (Sprite|SetFlipbook (Variables|Default|GetFlipBookAnimation) (Variables|PipeVisualSettings|GetAnimationFlipBook))
  (Rendering|Components|Sprite|SetSprite (Variables|Default|GetSpriteImage) (Variables|PipeVisualSettings|GetImageSprite))
  (Variables|Default|SetTopGateRef (Variables|Default|GetTopGate)))