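; RotatingRing is a level actor that spins on its pitch axis through a RotatingMovement component.
; The construction script feeds the RotationRate variable into that component and snaps the actor to world Y zero, keeping its X and Z.
; On a hit flagged as an initial overlap, it applies a small negative damage value to the other actor, with itself as causer.
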(event Collision|EventHit
  (params (MyComp :type Primitive%20Component%20Object%20Reference) (Other :type Actor%20Object%20Reference) (OtherComp :type Primitive%20Component%20Object%20Reference) (bSelfMoved :type Boolean) (HitLocation :type Vector :default "0, 0, 0") (HitNormal :type Vector :default "0, 0, 0") (NormalImpulse :type Vector :default "0, 0, 0") (Hit :type Hit%20Result%20Structure%20%28by%20ref%29))
  (if (.bInitialOverlap (Collision|BreakHitResult Hit))
    (Game|Damage|ApplyDamage Other -0.1 0 self)))

(fn ConstructionScript
  (bind _returnvalue (Transformation|GetActorLocation))
  (bind (_x _y _z) (Math|Vector|BreakVector _returnvalue))
  (Variables|/Script/Engine.RotatingMovementComponent|SetRotationRate (Variables|Default|GetRotatingMovement1) (Math|Rotator|MakeRotator 0.0 (Variables|Default|GetRotationRate) 0.0))
  (Transformation|SetActorLocation (Math|Vector|MakeVector _x 0.0 _z) false false))