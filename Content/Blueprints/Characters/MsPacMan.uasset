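; Ms. Pac-Man character Blueprint that switches its Paper2D sprite flipbook based on movement speed.
; The UpdateAnimation event measures velocity length, selecting the RunIdle flipbook above a speed threshold and RunIdleUp otherwise, including when stationary.
; Nothing in this graph calls UpdateAnimation; BeginPlay, Tick and overlap events are disabled stubs, and the construction script only calls its parent.
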(event Custom|UpdateAnimation
  (bind _returnvalue (Transformation|GetVelocity))
  (bind _returnvalue_2 (Math|Vector|VectorLength _returnvalue))
  ;[1 1 1] Handle Animation
  (Sprite|SetFlipbook (Variables|Default|GetSprite) (select (> _returnvalue_2 0.0) (select (> _returnvalue_2 5.5e+02) "/Game/Assets/MsPacMan/MsPacManRunIdle_MsPacManRunIdle.MsPacManRunIdle_MsPacManRunIdle" "/Game/Assets/MsPacMan/MsPacManRunIdleUp_MsPacManRunIdleUp.MsPacManRunIdleUp_MsPacManRunIdleUp") "/Game/Assets/MsPacMan/MsPacManRunIdleUp_MsPacManRunIdleUp.MsPacManRunIdleUp_MsPacManRunIdleUp")))

(event EventBeginPlay
  (|CallParentFunction))

(event Collision|EventActorBeginOverlap
  (params (OtherActor :type Actor%20Object%20Reference)))

(event EventTick
  (params (DeltaSeconds :type Float%20%28single-precision%29))
  (|CallParentFunction 0.0))

(fn ConstructionScript
  (|CallParentFunction))