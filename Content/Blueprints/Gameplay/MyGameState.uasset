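; GameState Blueprint that runs the match countdown for the current map.
; On BeginPlay a looping one-second timer calls UpdateGameTime, which subtracts a second from MapPlayTime stored on the GameInfoInstance game instance.
; When under a second remains it clears the timer and prints Game OVER; the actual game-over trigger is marked unfinished.
; A GetMyID event prints a given player controller's ID for debugging.
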(event Custom|UpdateGameTime
  (bind _asgame_info_instance (Utilities|Casting|CastToGameInfoInstance (Game|GetGameInstance)))
  (bind _output_get (Variables|/Game/Blueprints/AllLevels/GameInfoInstance.GameInfoInstance_C|SetMapPlayTime _asgame_info_instance (- (Variables|/Game/Blueprints/AllLevels/GameInfoInstance.GameInfoInstance_C|GetMapPlayTime _asgame_info_instance) (Math|Timespan|MakeTimespan 0 0 0 1))))
  (if (< _output_get (Math|Timespan|MakeTimespan 0 0 0 1))
    ;[1 1 1] Game Over Trigger - Need to complete
    (Utilities|Time|ClearandInvalidateTimerbyHandle (stale EventBeginPlay _returnvalue))
    (Development|PrintString "Game OVER" true true "(R=0.000000,G=0.660000,B=1.000000,A=1.000000)" 2e+01)))

(event Custom|GetMyID
  (params (ThePlayerController :type Player%20Controller%20Object%20Reference))
  (bind _returnvalue (Class|GameplayStatics|GetPlayerControllerID ThePlayerController))
  (Development|PrintString (Utilities|String|Append "GM GetMyID, Player Controller ID: " (Utilities|String|ToString(Integer) _returnvalue)) true true "(R=0.000000,G=0.660000,B=1.000000,A=1.000000)" 1e+01))

(event EventBeginPlay
  (Development|PrintString "MyGameState : Event BeginPlay" true true "(R=0.000000,G=0.660000,B=1.000000,A=1.000000)" 2e+01)
  (bind _returnvalue (Utilities|Time|SetTimerbyFunctionName 0 "UpdateGameTime" 1.0 true)))

(event EventTick
  (params (DeltaSeconds :type Float%20%28single-precision%29)))

(fn ConstructionScript)